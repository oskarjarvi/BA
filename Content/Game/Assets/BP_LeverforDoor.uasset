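; Lever trigger Blueprint that opens a linked door, DoorSelect, in two stages through two collision boxes.
; The first overlap on either box opens the door halfway, clears IsClosed and records which box fired.
; A later overlap on the opposite box opens it all the way.
; Overlaps are not filtered by actor, and the state flags are never reset here.
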(event `self.Collision Box1.OnComponentBeginOverlap`
  (params (OverlappedComponent :type "PrimitiveComponent Object Reference") (OtherActor :type "Actor Object Reference") (OtherComp :type "PrimitiveComponent Object Reference") (OtherBodyIndex :type Integer) (bFromSweep :type Boolean) (SweepResult :type "HitResult Structure (by ref)"))
  (if (`self.IsClosed`)
    (`/Game/Game/Assets/BP_Door.OpeningDoorHalfway` (`self.DoorSelect`))
    (set `self.IsClosed` false)
    (set `self.HaveBeen1` true)
    (elif (`self.HaveBeen2`)
      (`/Game/Game/Assets/BP_Door.OpeningAllTheWay` (`self.DoorSelect`)))))

(event `self.Collision Box2.OnComponentBeginOverlap`
  (params (OverlappedComponent :type "PrimitiveComponent Object Reference") (OtherActor :type "Actor Object Reference") (OtherComp :type "PrimitiveComponent Object Reference") (OtherBodyIndex :type Integer) (bFromSweep :type Boolean) (SweepResult :type "HitResult Structure (by ref)"))
  (if (`self.IsClosed`)
    (`/Game/Game/Assets/BP_Door.OpeningDoorHalfway` (`self.DoorSelect`))
    (set `self.IsClosed` false)
    (set `self.HaveBeen2` true)
    (elif (`self.HaveBeen1`)
      (`/Game/Game/Assets/BP_Door.OpeningAllTheWay` (`self.DoorSelect`)))))

(fn `UserConstructionScript`)