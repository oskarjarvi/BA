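; Drawbridge interactive that rotates its bridge toward a target rotation as counterweights are cut, extending a parent counterweight Blueprint.
; Each cut picks an intermediate rotation using the step percentage times the cut count, blending from the stored start rotation to the target.
; A timeline's HeightLift track animates the bridge there.
; On finish, the reached rotation becomes the start for the next cut, so each blend covers the remaining arc.
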(event `self.ReceiveBeginPlay`
  (`parent.ReceiveBeginPlay`)
  (set `self.InitialRotation` (`SceneComponent.RelativeRotation` (`self.Bridge`))))

(event `self.CounterweightCut`
  (`parent.CounterweightCut`)
  (set `self.NewTargetRotation` (`KismetMathLibrary.RLerp` (`self.InitialRotation`) (`self.TargetRotation`) (* (`self.StepPercentage`) (`self.CounterweightsCut`))))
  (bind (_direction _heightlift) (`Timeline|Timeline` :!via `PlayFromStart`)
    (:`Update`
      (`SceneComponent.K2_SetRelativeRotation` (`self.Bridge`) (`KismetMathLibrary.RLerp` (`self.InitialRotation`) (`self.NewTargetRotation`) _heightlift) false false))
    (:`Finished`
      (set `self.InitialRotation` (`SceneComponent.RelativeRotation` (`self.Bridge`))))))

(fn `UserConstructionScript`
  (`parent.UserConstructionScript`))