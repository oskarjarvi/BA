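; BP_LiftingGate is a gate that lifts toward a target location as its counterweights are cut, building on a parent class's counterweight event.
; Each cut computes a new target from the current start location, the remaining offset to TargetLocation, StepPercentage and the CounterweightsCut count.
; The LiftDoor timeline lerps the Gate's relative location to that point, then saves it as the next start location when finished.
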(event `self.ReceiveBeginPlay`
  (`parent.ReceiveBeginPlay`)
  (set `self.InitialLocation` (`SceneComponent.RelativeLocation` (`self.Gate`))))

(event `self.CounterweightCut`
  (bind _initiallocation (`self.InitialLocation`))
  (`parent.CounterweightCut`)
  (set `self.NewTargetPosition` (+ _initiallocation (* (* (- (`self.TargetLocation`) _initiallocation) (`self.StepPercentage`)) (`self.CounterweightsCut`))))
  (bind (_direction _heightlift) (`Timeline|LiftDoor` :!via `PlayFromStart`)
    (:`Update`
      (`SceneComponent.K2_SetRelativeLocation` (`self.Gate`) (`KismetMathLibrary.VLerp` (`self.InitialLocation`) (`self.NewTargetPosition`) _heightlift) false false))
    (:`Finished`
      (set `self.InitialLocation` (`SceneComponent.RelativeLocation` (`self.Gate`))))))

(fn `UserConstructionScript`
  (`parent.UserConstructionScript`))