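; Base Blueprint for an interactive door linked to a set of counterweights that can be cut.
; On BeginPlay it binds to each valid counterweight's cut event, counts them, and derives an equal step percentage per counterweight.
; Each cut event increments a running count; this Blueprint itself contains no door movement logic.
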(event `self.ReceiveBeginPlay`
  (for _array_element (`self.CounterWeights`)
    (`/Engine/EditorBlueprintResources/StandardMacros.IsValid` _array_element
      (:`Is Valid`
        (add `/Game/Game/Assets/Interactive_Environments/BP_CounterWeight.OnCounterWeightCut` _array_element (delegate `CounterweightCut`))
        (`/Engine/EditorBlueprintResources/StandardMacros.IncrementFloat` (`self.ValidCounterweights`)))))
  (set `self.StepPercentage` (/ 1.0 (`self.ValidCounterweights`))))

(event `CounterweightCut`
  (`/Engine/EditorBlueprintResources/StandardMacros.IncrementFloat` (`self.CounterweightsCut`)))

(fn `UserConstructionScript`)