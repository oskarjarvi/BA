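; BP_InteractiveDoor is an interactive environment gate that opens once all its linked counterweights are cut.
; On BeginPlay it binds to each counterweight's cut event, caches the gate's starting transform and applies an optional mesh override.
; A cut counter fires a timeline when it reaches the counterweight count.
; The timeline animates the gate by AnimType: lifting it, rolling it as a winding bridge, or sliding it.
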(event `self.ReceiveBeginPlay`
  (for _array_element (`self.CounterWeights`)
    (add `/Game/Game/Assets/Interactive_Environments/BP_CounterWeight.OnCounterWeightCut` _array_element (`|CreateDelegate` :!event `CounterWeightCut`))
    (set `self.InitialLocation` (`SceneComponent.RelativeLocation` (`self.Gate`)))
    (set `self.InitialRotation` (`self.K2_GetActorRotation`))
    (bind _gatemesh (`self.GateMesh`)
      (:`then`
        (`StaticMeshComponent.SetStaticMesh` (`self.Gate`) _gatemesh))
      (:`else`))))

(event `CounterWeightCut`
  (bind _returnvalue (`KismetArrayLibrary.Array_Length` (`self.CounterWeights`)))
  (bind _result (`/Engine/EditorBlueprintResources/StandardMacros.IncrementInt` (`self.CounterweightsCut`))
    (:`  `
      (if (== (`KismetMathLibrary.Clamp` _result 0 _returnvalue) _returnvalue)
        (`self.TriggerAnimation`)))))

(event `TriggerAnimation`
  (bind _initiallocation (`self.InitialLocation`))
  (bind _gate (`self.Gate`))
  (bind _initiallocation_2 (`self.InitialLocation`))
  (bind (_direction _progress) (`Timeline|InteractiveDoorAnim` :!via `PlayFromStart`)
    (:`Update`
      (switch `/Game/Game/Assets/Interactive_Environments/E_InteractiveDoorAnimType` (`self.AnimType`)
        (:`NewEnumerator0`
          (`SceneComponent.K2_SetRelativeLocation` _gate (`KismetMathLibrary.VLerp` _initiallocation_2 (+ _initiallocation_2 (* (`KismetMathLibrary.GetUpVector` (struct)) (`self.LiftHeight`))) _progress) false false))
        (:`NewEnumerator1`
          (`SceneComponent.K2_SetRelativeRotation` _gate (`KismetMathLibrary.ComposeRotators` (`self.InitialRotation`) (`KismetMathLibrary.MakeRotator` (* _progress (`self.RotationAmount`)))) false false))
        (:`NewEnumerator2`
          (`SceneComponent.K2_SetRelativeLocation` _gate (`KismetMathLibrary.VLerp` _initiallocation (+ _initiallocation (`self.SlideDistance`)) _progress) false false))))))

(fn `UserConstructionScript`)