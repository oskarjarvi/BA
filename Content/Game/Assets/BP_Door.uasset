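; BP_Door is a door actor that moves open in two stages, each triggered by its own custom event.
; BeginPlay caches the start location, then the halfway timeline offsets the door from it by an animated vector and stores the result in NewLocation.
; The all-the-way timeline adds its own vector to that stored position, so the second stage continues from where the first left off.
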(event `self.ReceiveBeginPlay`
  (set `self.StartLocation` (`self.K2_GetActorLocation`)))

(event `OpeningDoorHalfway`
  (bind (_direction _halfwayvector) (`Timeline|DoorHalfway` :!via `PlayFromStart`)
    (:`Update`
      (bind _returnvalue (+ (`self.StartLocation`) _halfwayvector))
      (`self.K2_SetActorLocation` _returnvalue)
      (set `self.NewLocation` _returnvalue))))

(event `OpeningAllTheWay`
  (bind (_direction _dooralltheway) (`Timeline|DoorAllTheWay`)
    (:`Update`
      (`self.K2_SetActorLocation` (+ (`self.NewLocation`) _dooralltheway)))))

(fn `UserConstructionScript`)