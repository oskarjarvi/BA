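; BP_RoofTrigger is a trigger actor that hides a referenced static mesh, by its name a roof, while the player is inside it.
; When a PlayerCharacter begins overlapping, it hides the mesh component and turns off its collision.
; When the overlap ends, it shows the mesh again but leaves collision disabled.
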(event `self.ReceiveBeginPlay`)

(event `self.ReceiveActorBeginOverlap`
  (params (OtherActor :type "Actor Object Reference"))
  (bind _staticmesh (`self.StaticMesh`))
  (cast `/Game/Game/Characters/Player/PlayerCharacter` OtherActor)
  (`SceneComponent.SetVisibility` (`/Game/Game/Assets/BP_Roof.StaticMesh` _staticmesh) false false)
  (`PrimitiveComponent.SetCollisionEnabled` (`/Game/Game/Assets/BP_Roof.StaticMesh` _staticmesh) "NoCollision"))

(event `self.ReceiveActorEndOverlap`
  (params (OtherActor :type "Actor Object Reference"))
  (cast `/Game/Game/Characters/Player/PlayerCharacter` OtherActor)
  (`SceneComponent.SetVisibility` (`/Game/Game/Assets/BP_Roof.StaticMesh` (`self.StaticMesh`)) true false))

(fn `UserConstructionScript`)