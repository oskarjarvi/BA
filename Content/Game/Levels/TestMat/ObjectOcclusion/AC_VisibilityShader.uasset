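; Actor component that toggles an occlusion shader when something blocks the view ahead of its owner's tagged camera.
; Each tick it finds that camera and line traces forward on the Visibility channel up to a configurable distance.
; A hit interpolates the AllowOcclusionShader scalar in MPC_CameraVector toward one at constant speed, and a miss toward zero.
; The shared material parameter collection passes this fade value to materials.
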(event `self.ReceiveTick`
  (params (DeltaSeconds :type "Float (single-precision)"))
  (bind _output (`|GetArrayItem` (`Actor.GetComponentsByTag` (`self.GetOwner`) "/Script/Engine.CameraComponent" (`self.Camera Tag`))))
  (bind _returnvalue (`SceneComponent.K2_GetComponentLocation` _output))
  ;[1 1 1] Checks if the camera has hit the object and then allows the shader to activate
  (`/Engine/EditorBlueprintResources/StandardMacros.IsValid` _output
    (:`Is Valid`
      (bind (_outhit _returnvalue_2) (`KismetSystemLibrary.LineTraceSingle` :`Start` _returnvalue :`End` (+ _returnvalue (* (`SceneComponent.GetForwardVector` _output) (`self.Distance for occlusion`))) :`TraceChannel` "TraceTypeQuery1" :`DrawDebugType` (`self.Draw Debug Type`)))
      (if _returnvalue_2
        (bind _returnvalue_3 (`KismetMaterialLibrary.GetScalarParameterValue` "/Game/Game/Levels/TestMat/ObjectOcclusion/MPC_CameraVector.MPC_CameraVector" "AllowOcclusionShader"))
        (`KismetMaterialLibrary.SetScalarParameterValue` "/Game/Game/Levels/TestMat/ObjectOcclusion/MPC_CameraVector.MPC_CameraVector" "AllowOcclusionShader" (`KismetMathLibrary.FInterpTo_Constant` _returnvalue_3 1.0 (`GameplayStatics.GetWorldDeltaSeconds`) (* (`self.Interp Speed`) 100.0)))
        (else
          (bind _returnvalue_4 (`KismetMaterialLibrary.GetScalarParameterValue` "/Game/Game/Levels/TestMat/ObjectOcclusion/MPC_CameraVector.MPC_CameraVector" "AllowOcclusionShader"))
          (`KismetMaterialLibrary.SetScalarParameterValue` "/Game/Game/Levels/TestMat/ObjectOcclusion/MPC_CameraVector.MPC_CameraVector" "AllowOcclusionShader" (`KismetMathLibrary.FInterpTo_Constant` _returnvalue_4 0.0 (`GameplayStatics.GetWorldDeltaSeconds`) (* (`self.Interp Speed`) 100.0))))))))