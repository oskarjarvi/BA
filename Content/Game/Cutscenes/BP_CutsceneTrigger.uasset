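; BP_CutsceneTrigger is a trigger actor that plays a cutscene once when the player character enters it.
; On BeginPlay it creates a level sequence player from its CutsceneSequence and stores it.
; The first overlap passes a DoOnce, casts to PlayerCharacter, disables input, plays the sequence, and re-enables input after a delay matching its duration.
; Because DoOnce precedes the cast, an overlap by any other actor consumes the single trigger.
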(event `self.ReceiveBeginPlay`
  (bind (_outactor _returnvalue) (`LevelSequencePlayer.CreateLevelSequencePlayer` (`self.CutsceneSequence`)))
  (set `self.SequenceRef` _returnvalue))

(event `self.ReceiveActorBeginOverlap`
  (params (OtherActor :type "Actor Object Reference"))
  (bind _sequenceref (`self.SequenceRef`))
  (`/Engine/EditorBlueprintResources/StandardMacros.DoOnce` false
    (:`Completed`
      (bind _asplayer_character (cast `/Game/Game/Characters/Player/PlayerCharacter` OtherActor))
      (`self.DisableInput` _asplayer_character null)
      (`MovieSceneSequencePlayer.Play` _sequenceref)
      (`KismetSystemLibrary.Delay` (`TimeManagementBlueprintLibrary.Conv_QualifiedFrameTimeToSeconds` (`MovieSceneSequencePlayer.GetDuration` _sequenceref)))
      (`self.EnableInput` _asplayer_character null))))

(fn `UserConstructionScript`)