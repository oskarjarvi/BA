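; BP_HealingOrb is a pickup actor that heals the player on touch.
; When a PlayerCharacter overlaps its Box, it calls Heal with HealAmount, plays an optional heal sound at its location and destroys itself.
; The Destroyed event plays a separate absorb sound, so that sound follows any destruction of the orb.
; A DebugSphereVisible flag assigns an editor sphere mesh to TestObject on BeginPlay.
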(event `self.ReceiveBeginPlay`
  (if (`self.DebugSphereVisible`)
    (`StaticMeshComponent.SetStaticMesh` (`self.TestObject`) "/Engine/EditorMeshes/EditorSphere.EditorSphere")))

(event `self.Box.OnComponentBeginOverlap`
  (params (OverlappedComponent :type "PrimitiveComponent Object Reference") (OtherActor :type "Actor Object Reference") (OtherComp :type "PrimitiveComponent Object Reference") (OtherBodyIndex :type Integer) (bFromSweep :type Boolean) (SweepResult :type "HitResult Structure (by ref)"))
  (bind _asplayer_character (cast `/Game/Game/Characters/Player/PlayerCharacter` OtherActor))
  (`/Game/Game/DamageSystem/BPI_Damageable.Heal` _asplayer_character (`self.HealAmount`))
  (bind _healsound (`self.HealSound`)
    (:`then`
      (`GameplayStatics.PlaySoundAtLocation` _healsound (`self.K2_GetActorLocation`) (struct) 1.0 1.0 0.0 null null null null))
    (:`else`
      _))
  (`self.K2_DestroyActor`))

(event `self.ReceiveDestroyed`
  (`GameplayStatics.PlaySoundAtLocation` (`self.HealthAbsorbSound`) (`self.K2_GetActorLocation`) (struct) 1.0 1.0 0.0 null null null null))

(fn `UserConstructionScript`)