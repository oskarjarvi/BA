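; Damage system component that manages health, death, blocking and a pool of attack tokens for its owner.
; TakeDamage routes each DamageInfo through the CanBeDamaged macro, which resolves to block, damage or no damage from death, invincibility and blocking state.
; Results fire dispatchers for blocks, death and damage responses, the last only when interruptible or forced.
; Heal clamps health while alive, and attack tokens are reserved and returned by amount.
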(fn `GetCurrentHealth`
  (returns (Health :type "Float (double-precision)"))
  (return 0.0))

(fn `GetMaxHealth`
  (returns (MaxHealth :type "Float (double-precision)"))
  (return 0.0))

(fn `Heal`
  (params (Amount :type "Float (double-precision)" :default 0.0))
  (returns (NewHealth :type "Float (double-precision)"))
  (if (not (`self.IsDead`))
    (set `self.Health` (`KismetMathLibrary.FClamp` (+ (`self.Health`) Amount) 0.0 (`self.MaxHealth`)))
    (return 0.0)))

(fn `ReserveAttackToken`
  (params (Amount :type Integer))
  (returns (Success :type Boolean))
  (if (>= (`self.AvailableAttackTokens`) Amount)
    (set `self.AvailableAttackTokens` (- (`self.AvailableAttackTokens`) Amount))
    (return true)
    (else
      (return false))))

(fn `ReturnAttackToken`
  (params (Amount :type Integer))
  (set `self.AvailableAttackTokens` (+ (`self.AvailableAttackTokens`) Amount))
  (return))

(fn `TakeDamage`
  (params (DamageInfo :type "/Game/Game/DamageSystem/S_DamageInfo Structure") (DamageCauser :type "Actor Object Reference"))
  (returns (WasDamaged :type Boolean))
  (bind (_amount _damagetype _damageresponse _shoulddamageinvincible _canbeblocked _canbeparried _shouldforceinterrupt) (break `/Game/Game/DamageSystem/S_DamageInfo` DamageInfo))
  (`self.CanBeDamaged` _shoulddamageinvincible _canbeblocked
    (:`BlockDamage`
      (`self.OnBlocked` _canbeparried)
      (return false))
    (:`DoDamage`
      (bind _output_get (set `self.Health` (- (`self.Health`) _amount)))
      (if (<= _output_get 0.0)
        (set `self.IsDead` true)
        (`self.OnDeath`)
        (elif (or (`self.IsInteruptible`) _shouldforceinterrupt)
          (`self.OnDamageResponse` _damageresponse DamageCauser)))
      (return false))
    (:`NoDamage`
      (return false))))