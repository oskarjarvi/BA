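; Bomb projectile that is lobbed on a calculated arc from its owner toward a Target actor and explodes after coming to rest.
; After a collision hit, a looping timer checks for near-zero velocity, then spawns a circle effect and starts the fuse.
; When the fuse ends, it broadcasts OnBombExplosion with its location, plays effect and sound, and destroys itself.
; The construction script gives the mesh a dynamic material instance.
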(event `self.ReceiveBeginPlay`
  (bind _boxcollision (`self.BoxCollision`))
  (`parent.ReceiveBeginPlay`)
  (`PrimitiveComponent.SetCollisionResponseToChannel` _boxcollision "ECC_GameTraceChannel2" "ECR_Ignore")
  (`PrimitiveComponent.SetCollisionResponseToChannel` _boxcollision "ECC_GameTraceChannel3" "ECR_Ignore")
  (bind _outlaunchvelocity (`GameplayStatics.SuggestProjectileVelocity_CustomArc` (`self.K2_GetActorLocation` (`self.GetOwner`)) (`self.K2_GetActorLocation` (`self.Target`))))
  (set `MovementComponent.Velocity` _outlaunchvelocity (`self.ProjectileMovement`)))

(event `self.BoxCollision.OnComponentHit`
  (params (HitComponent :type "PrimitiveComponent Object Reference") (OtherActor :type "Actor Object Reference") (OtherComp :type "PrimitiveComponent Object Reference") (NormalImpulse :type "Vector Structure") (Hit :type "HitResult Structure (by ref)"))
  (bind _returnvalue (`KismetSystemLibrary.K2_SetTimerDelegate` (delegate `CheckIfStopped`) 0.2 true))
  (set `self.CheckTimer` _returnvalue))

(event `CheckIfStopped`
  (if (`KismetMathLibrary.Vector_IsNearlyZero` (`MovementComponent.Velocity` (`self.ProjectileMovement`)) 1.0)
    (`KismetSystemLibrary.K2_ClearAndInvalidateTimerHandle` (`self.CheckTimer`))
    (`NiagaraFunctionLibrary.SpawnSystemAtLocation` "/Game/Game/VFXs/NS_BombCircle.NS_BombCircle" (`self.K2_GetActorLocation`))
    (`KismetSystemLibrary.K2_SetTimerDelegate` (delegate `StartExplosionFuse`) (`self.ExplosionTime`))))

(event `StartExplosionFuse`
  (bind _returnvalue (`self.K2_GetActorLocation`))
  (`self.OnBombExplosion` _returnvalue)
  (`NiagaraFunctionLibrary.SpawnSystemAtLocation` (`self.ExplosionEffect`) _returnvalue)
  (`GameplayStatics.PlaySoundAtLocation` (`self.BombExplosionSound`) _returnvalue (struct) 1.0 1.0 0.0 null null null null)
  (`self.K2_DestroyActor`))

(event `OnBombExplosion_Event` :!signature `self.OnBombExplosion`
  (params (ExplosionLocation :type "Vector Structure")))

(fn `UserConstructionScript`
  (bind _mesh (`self.Mesh`))
  (`parent.UserConstructionScript`)
  (bind _returnvalue (`PrimitiveComponent.CreateDynamicMaterialInstance` _mesh 0 (`PrimitiveComponent.GetMaterial` _mesh 0) "None"))
  (bind _output_get (set `self.MatInst` _returnvalue))
  (`PrimitiveComponent.SetMaterial` _mesh 0 _output_get))