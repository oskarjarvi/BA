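; Sword weapon Blueprint that deals fixed damage to any actor it overlaps, except the first player's character.
; Each overlap reports an AI damage-sense event at the sword's location, with the owner as instigator.
; It then sends the hit actor a damage-info message and activates blood and spark effects without resetting them.
; The construction script only calls its parent.
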(event `self.ReceiveActorBeginOverlap`
  (params (OtherActor :type "Actor Object Reference"))
  (bind _returnvalue (`self.GetOwner`))
  (if (!= OtherActor (`GameplayStatics.GetPlayerCharacter` 0))
    (`AISense_Damage.ReportDamageEvent` OtherActor _returnvalue 35.0 (`self.K2_GetActorLocation`))
    (message `/Game/Game/DamageSystem/BPI_Damageable.TakeDamage` OtherActor (make `/Game/Game/DamageSystem/S_DamageInfo` 35.0 "NewEnumerator1" "NewEnumerator1") _returnvalue)
    ;[1 1 1] Bloodsplatter Activate
    (`ActorComponent.Activate` (`self.NS_Blood`) false)
    (`ActorComponent.Activate` (`self.NS_Spark`) false)))

(fn `UserConstructionScript`
  (`parent.UserConstructionScript`))