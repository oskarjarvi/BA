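; Princess sword weapon Blueprint that turns box overlaps into enemy hits or shield blocks.
; Overlapping a component tagged Shield spawns the spark effect and calls the weapon-blocked event.
; Otherwise, an overlapped BP_Enemy_Base sets HitLocation to its actor location, spawns the spark and calls the weapon-hit event.
; The blocked path does not update HitLocation, so its spark uses the previously stored position.
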(event `Spawn Spark`
  (`NiagaraFunctionLibrary.SpawnSystemAtLocation` (`self.HitEffect`) (`self.HitLocation`)))

(event `self.Box.OnComponentBeginOverlap`
  (params (OverlappedComponent :type "PrimitiveComponent Object Reference") (OtherActor :type "Actor Object Reference") (OtherComp :type "PrimitiveComponent Object Reference") (OtherBodyIndex :type Integer) (bFromSweep :type Boolean) (SweepResult :type "HitResult Structure (by ref)"))
  (if (`ActorComponent.ComponentHasTag` OtherComp "Shield")
    (`self.Spawn Spark`)
    (`self.OnWeaponBlocked`)
    (else
      (bind _asbp_enemy_base (cast `/Game/Game/Characters/Enemy/BP_Enemy_Base` OtherActor))
      (bind _output_get (set `self.HitLocation` (`self.K2_GetActorLocation` _asbp_enemy_base)))
      (`self.Spawn Spark`)
      (`self.OnWeaponHit` _asbp_enemy_base _output_get))))

(fn `UserConstructionScript`
  (`parent.UserConstructionScript`))