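; Arrow projectile actor that flies when fired, sticks to what it hits and despawns.
; Fire adds a ProjectileMovement component at runtime, enables Box collision and uses the passed Direction directly as velocity.
; Hit compares the other component to the player character, then stops movement, sets rotation from velocity (read after the stop) and attaches with world transform kept.
; Collision is then disabled and the arrow is destroyed after DespawnTimer.
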(event `Fire`
  (params (Direction :type "Vector Structure"))
  ;[1 1 1] Fire Arrow
  (bind _returnvalue (`AddComponent|NODE_AddProjectileMovementComponent-0`))
  (bind _output_get (set `self.ProjectileMovementRef` _returnvalue))
  (`PrimitiveComponent.SetCollisionEnabled` (`self.Box`) "QueryAndPhysics")
  (set `MovementComponent.Velocity` Direction _output_get))

(event `self.ReceiveHit`
  (params (MyComp :type "PrimitiveComponent Object Reference") (Other :type "Actor Object Reference") (OtherComp :type "PrimitiveComponent Object Reference") (bSelfMoved :type Boolean) (HitLocation :type "Vector Structure") (HitNormal :type "Vector Structure") (NormalImpulse :type "Vector Structure") (Hit :type "HitResult Structure (by ref)"))
  (bind _projectilemovementref (`self.ProjectileMovementRef`))
  ;[1 1 1] Attach to anything that is not player
  (if (not (== OtherComp (`GameplayStatics.GetPlayerCharacter` 0)))
    (`MovementComponent.StopMovementImmediately` _projectilemovementref)
    (`self.K2_SetActorRotation` (`KismetMathLibrary.MakeRotFromX` (`MovementComponent.Velocity` _projectilemovementref)))
    (`self.K2_AttachToComponent` OtherComp "None" "KeepWorld" "KeepWorld" "KeepWorld")
    (`PrimitiveComponent.SetCollisionEnabled` (`self.Box`) "NoCollision")
    (`KismetSystemLibrary.Delay` (`self.DespawnTimer`))
    (`self.K2_DestroyActor`)))

(fn `UserConstructionScript`)