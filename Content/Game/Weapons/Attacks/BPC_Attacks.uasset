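; Attack component that spawns an owner's fire arrow and dark energy spell projectiles and resolves their hits.
; SpawnAndAttachProjectile spawns a targeted arrow and, given a valid parent component, snaps it to a socket and binds its impact through FireArrow.
; MagicSpell spawns a targeted dark energy projectile and binds its impact.
; Both impact handlers send damage by message, report an AI damage event and broadcast OnAttackEnded.
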(event `FireArrow`
  (params (DamageInfo :type "/Game/Game/DamageSystem/S_DamageInfo Structure") (ArrowRef :type "/Game/Game/Weapons/Projectiles/BP_Projectile_FireArrow Object Reference"))
  (add `/Game/Game/Weapons/Projectiles/BP_Projectile_Base.OnProjectileImpact` ArrowRef (delegate `OnArrowHit`)))

(event `OnArrowHit`
  (params (OtherActor :type "Actor Object Reference") (Hit :type "HitResult Structure"))
  (bind _returnvalue (`self.GetOwner`))
  (message `/Game/Game/DamageSystem/BPI_Damageable.TakeDamage` OtherActor (stale `FireArrow` DamageInfo) _returnvalue)
  (`AISense_Damage.ReportDamageEvent` OtherActor _returnvalue (`.Amount_2_73F035C74537F3836B18D6A4FF619D19` (break `/Game/Game/DamageSystem/S_DamageInfo` (stale `FireArrow` DamageInfo))) (`Actor.K2_GetActorLocation` (`self.GetOwner`)))
  (`self.OnAttackEnded`))

(event `MagicSpell`
  (params (SpawnTransform :type "Transform Structure") (Target :type "Actor Object Reference") (DamageInfo :type "/Game/Game/DamageSystem/S_DamageInfo Structure"))
  (bind _returnvalue (`|SpawnActorFromClass` "/Game/Game/Weapons/Projectiles/BP_Projectile_DarkEnergy.BP_Projectile_DarkEnergy_C" SpawnTransform "Undefined" "MultiplyWithRoot" (`self.GetOwner`) 1000.0 0.0 Target true null))
  (add `/Game/Game/Weapons/Projectiles/BP_Projectile_Base.OnProjectileImpact` _returnvalue (delegate `OnProjectileHit`))
  (`PrimitiveComponent.IgnoreActorWhenMoving` (`/Game/Game/Weapons/Projectiles/BP_Projectile_Base.BoxCollision` _returnvalue) _returnvalue true))

(event `OnProjectileHit`
  (params (OtherActor :type "Actor Object Reference") (Hit :type "HitResult Structure"))
  (bind _returnvalue (`self.GetOwner`))
  (message `/Game/Game/DamageSystem/BPI_Damageable.TakeDamage` OtherActor (stale `MagicSpell` DamageInfo) _returnvalue)
  (`AISense_Damage.ReportDamageEvent` OtherActor _returnvalue (`.Amount_2_73F035C74537F3836B18D6A4FF619D19` (break `/Game/Game/DamageSystem/S_DamageInfo` (stale `MagicSpell` DamageInfo))) (`Actor.K2_GetActorLocation` (`self.GetOwner`)))
  (`self.OnAttackEnded`))

(fn `SpawnAndAttachProjectile`
  (params (SpawnTransform :type "Transform Structure") (AttachToComponent :type "SceneComponent Object Reference") (SocketName :type Name) (FlyOnSpawn :type Boolean) (DamageInfo :type "/Game/Game/DamageSystem/S_DamageInfo Structure") (AttackTarget :type "Actor Object Reference"))
  (returns (ProjectileRef :type "/Game/Game/Weapons/Projectiles/BP_Projectile_FireArrow Object Reference"))
  (bind _returnvalue (`|SpawnActorFromClass` "/Game/Game/Weapons/Projectiles/BP_Projectile_FireArrow.BP_Projectile_FireArrow_C" SpawnTransform "Undefined" "MultiplyWithRoot" (`self.GetOwner`) 500.0 0.0 AttackTarget FlyOnSpawn null))
  (`/Engine/EditorBlueprintResources/StandardMacros.IsValid` AttachToComponent
    (:`Is Valid`
      (`Actor.K2_AttachToComponent` _returnvalue AttachToComponent SocketName "SnapToTarget" "SnapToTarget" "SnapToTarget" true)
      (`self.FireArrow` DamageInfo _returnvalue)
      (return _returnvalue))))