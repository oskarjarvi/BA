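; Melee enemy character that extends a parent enemy with sword equip, unequip and slash attack behavior.
; Montage notifies spawn the sword onto a hand socket or destroy it, and draw-sword playback toggles the damage system's interruptible flag.
; The slash notify runs a debug-drawn forward sphere trace that sends damage to the hit actor.
; Montage endings fire equip, unequip and attack-end callbacks, and GetIdealRange supplies attack and defend radii.
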(event `self.ReceiveBeginPlay`
  (`parent.ReceiveBeginPlay`))

(event `/Game/Game/Characters/Enemy/AI/BPI_EnemyAI.EquipWeapon`
  (bind _bpc_damagesystem (`self.BPC_DamageSystem`))
  ;[1 1 1] Equipping Weapon
  (bind _notifyname (`|PlayMontage` (`self.Mesh`) "/Game/Game/Animations/BaseEnemy/Anims/DrawSword_Montage.DrawSword_Montage")
    (:`then`
      (set `/Game/Game/DamageSystem/BPC_DamageSystem.IsInteruptible` false _bpc_damagesystem))
    (:`OnCompleted`
      (`self.OnWeaponEquipped` :!label _label)
      (set `/Game/Game/DamageSystem/BPC_DamageSystem.IsInteruptible` true _bpc_damagesystem))
    (:`OnInterrupted`
      (goto _label))
    (:`OnNotifyBegin`
      (switch `name` _notifyname
        (:`WieldSword`
          (bind _returnvalue (`|SpawnActorFromClass` "/Game/Game/Weapons/BP_Weapon_Sword.BP_Weapon_Sword_C" (`self.GetTransform`) "Undefined" "MultiplyWithRoot" null null))
          (bind _output_get (set `self.WeaponActor` _returnvalue))
          (`self.K2_AttachToComponent` _output_get (`self.Mesh`) "hand_r_sword_socket" "SnapToTarget" "SnapToTarget" "SnapToTarget" true)
          (set `self.IsWieldingWeapon` true))))))

(event `/Game/Game/Characters/Enemy/AI/BPI_EnemyAI.UnEquipWeapon`
  (bind _notifyname (`|PlayMontage` null "/Game/Game/Animations/BaseEnemy/Anims/SheathSword_Montage.SheathSword_Montage")
    (:`OnCompleted`
      (`self.OnWeaponUnequipped`))
    (:`OnNotifyBegin`
      (switch `name` _notifyname
        (:`UnequipSword`
          (`self.K2_DestroyActor` (`self.WeaponActor`))
          (set `self.IsWieldingWeapon` false))))))

(event `/Game/Game/Characters/Enemy/AI/BPI_EnemyAI.Attack`
  (bind _returnvalue (`self.K2_GetActorLocation`))
  (bind _notifyname (`|PlayMontage` (`self.Mesh`) "/Game/Game/Animations/BaseEnemy/Anims/SlashMontage2.SlashMontage2")
    (:`OnCompleted`
      (`self.OnAttackEnd` :!label _label_2))
    (:`OnInterrupted`
      (goto _label_2))
    (:`OnNotifyBegin`
      (switch `name` _notifyname
        (:`Slash`
          (bind (_outhit _returnvalue_2) (`KismetSystemLibrary.SphereTraceSingleForObjects` :`Start` _returnvalue :`End` (+ _returnvalue (* (`self.GetActorForwardVector`) 200.0)) :`Radius` 20.0 :`ObjectTypes` (`|MakeArray` "ObjectTypeQuery9" :!type "EObjectTypeQuery Enum") :`DrawDebugType` "ForDuration"))
          (if _returnvalue_2
            (message `/Game/Game/DamageSystem/BPI_Damageable.TakeDamage` (`.HitActor` (`GameplayStatics.BreakHitResult` _outhit)) (make `/Game/Game/DamageSystem/S_DamageInfo` 25.0 "NewEnumerator1") self)))))))

(fn `GetIdealRange`
  (returns (AttackRadius :type "Float (double-precision)") (DefendRadius :type "Float (double-precision)"))
  (return 100.0 300.0))

(fn `UserConstructionScript`
  (`parent.UserConstructionScript`))