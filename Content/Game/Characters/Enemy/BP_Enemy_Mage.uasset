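; BP_Enemy_Mage is the mage enemy character, a child Blueprint that specializes the parent enemy's attack, movement speeds and combat ranges.
; Attack calls the parent, then plays the spell montage; its notify-begin branch has no actions wired, so no spell effect happens here.
; SetMovementSpeed maps each movement state to a fixed speed, and GetIdealRange returns fixed attack and defend radii.
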(event `/Game/Game/Characters/Enemy/AI/BPI_EnemyAI.Attack`
  (params (AttackTarget :type "Actor Object Reference"))
  (`parent.Attack` AttackTarget)
  (bind _notifyname (`|PlayMontage` (`self.Mesh`) "/Game/Game/Animations/RangedEnemy/MageAnims/Montage_Mage_Spell.Montage_Mage_Spell")
    (:`OnNotifyBegin`
      (switch `name` _notifyname))))

(fn `GetIdealRange`
  (returns (AttackRadius :type "Float (double-precision)") (DefendRadius :type "Float (double-precision)"))
  (return 500.0 700.0))

(fn `SetMovementSpeed`
  (params (Speed :type "/Game/Game/Characters/Enemy/AI/Enums/E_MovementSpeed Enum" :default "NewEnumerator0"))
  (returns (SpeedValue :type "Float (double-precision)"))
  (return (select `/Game/Game/Characters/Enemy/AI/Enums/E_MovementSpeed` Speed :`NewEnumerator1` 150.0 :`NewEnumerator2` 250.0 :`NewEnumerator3` 400.0)))

(fn `UserConstructionScript`
  (`parent.UserConstructionScript`))