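; Boss enemy character that fights with an axe and extends a parent enemy class with a dedicated boss health bar widget.
; Construction sets damage-component health from MaxHealth; BeginPlay creates the widget, which TakeDamage refreshes after parent handling.
; Equip and unequip events spawn or destroy the socketed axe, but the equipped callback is unwired.
; Its combo attack delegates to the attacks component, and movement states map to walk speeds.
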(event `self.ReceiveBeginPlay`
  (bind _bpc_damagesystem (`self.BPC_DamageSystem`))
  ;[1 1 1] Health
  (`parent.ReceiveBeginPlay`)
  (`WidgetComponent.SetWidget` (`self.HealthBar`) null)
  (bind _returnvalue (`|CreateWidget` "/Game/Game/Widgets/W_BossHealthBar.W_BossHealthBar_C"))
  (bind _output_get (set `self.BossHealthbarWidgetRef` _returnvalue))
  (`/Game/Game/Widgets/W_BossHealthBar.UpdateHealthPercentage` _output_get (`/Game/Game/DamageSystem/BPC_DamageSystem.Health` _bpc_damagesystem) (`/Game/Game/DamageSystem/BPC_DamageSystem.MaxHealth` _bpc_damagesystem)))

(event `/Game/Game/Characters/Enemy/AI/BPI_EnemyAI.EquipWeapon`
  ;[1 1 1] Equip/ UnEquip Weapon
  (bind _returnvalue (`|SpawnActorFromClass` "/Game/Game/Combat/Weapons/BP_Weapon_Axe.BP_Weapon_Axe_C" (`KismetMathLibrary.MakeTransform` (0.0 0.0 0.0)) "Undefined" "MultiplyWithRoot" self null))
  (bind _output_get (set `self.WeaponActor` _returnvalue))
  (`self.K2_AttachToComponent` _output_get (`self.Mesh`) "hand_r_axe_socket" "SnapToTarget" "SnapToTarget" "SnapToTarget" true)
  (set `self.IsWieldingWeapon` true))

(event `/Game/Game/Characters/Enemy/AI/BPI_EnemyAI.UnEquipWeapon`
  ;[1 1 1] Equip/ UnEquip Weapon
  (set `self.IsWieldingWeapon` false)
  (`self.K2_DestroyActor` (`self.WeaponActor`))
  (`KismetSystemLibrary.DelayUntilNextTick`)
  (`self.OnWeaponUnequipped`))

(event `AttackCombo1`
  (params (AttackTarget :type "Actor Object Reference"))
  (`/Game/Game/Combat/Attacks/BPC_Attacks.PrimaryMeleeAttack` (`self.BPC_Attacks`) (make `/Game/Game/Combat/Attacks/S_AttackInfo` AttackTarget null (make `/Game/Game/DamageSystem/S_DamageInfo` 20.0 "NewEnumerator1" "NewEnumerator1" false true true)) 40.0 250.0))

(fn `SetMovementSpeed`
  (params (Speed :type "/Game/Game/Characters/Enemy/AI/Enums/E_MovementSpeed Enum" :default "NewEnumerator0"))
  (returns (SpeedValue :type "Float (double-precision)"))
  (bind _output_get (set `CharacterMovementComponent.MaxWalkSpeed` (select `/Game/Game/Characters/Enemy/AI/Enums/E_MovementSpeed` Speed :`NewEnumerator0` 0.0 :`NewEnumerator1` 100.0 :`NewEnumerator2` 200.0 :`NewEnumerator3` 350.0 :!type "Float (single-precision)") (`self.CharacterMovement`)))
  (return _output_get))

(fn `TakeDamage`
  (params (DamageInfo :type "/Game/Game/DamageSystem/S_DamageInfo Structure") (DamageCause :type "Actor Object Reference"))
  (returns (WasDamaged :type Boolean))
  (bind _bpc_damagesystem (`self.BPC_DamageSystem`))
  (bind _wasdamaged (`parent.TakeDamage` DamageInfo DamageCause))
  (`/Game/Game/Widgets/W_BossHealthBar.UpdateHealthPercentage` (`self.BossHealthbarWidgetRef`) (`/Game/Game/DamageSystem/BPC_DamageSystem.Health` _bpc_damagesystem) (`/Game/Game/DamageSystem/BPC_DamageSystem.MaxHealth` _bpc_damagesystem))
  (return _wasdamaged))

(fn `UserConstructionScript`
  (bind _bpc_damagesystem (`self.BPC_DamageSystem`))
  (`parent.UserConstructionScript`)
  (bind _output_get (set `/Game/Game/DamageSystem/BPC_DamageSystem.MaxHealth` (`self.Max Health`) _bpc_damagesystem))
  (set `/Game/Game/DamageSystem/BPC_DamageSystem.Health` _output_get _bpc_damagesystem))