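; BP_Enemy_Mage is a mage enemy Blueprint that supplies four attacks, per-state movement speeds and ideal attack and defend ranges.
; Basic spell, barrage and ground smash hand montage and damage info to the BPCAttacks component.
; MageBomb plays its own montage, spawns a delayed lightning-strike AOE actor on a notify, and damages overlapped actors from other teams through message calls.
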(event `MageBomb`
  (params (AttackTarget :type "Actor Object Reference"))
  ;[1 1 1] Attacks
  (`self.Attack` AttackTarget)
  (bind _notifyname (`|PlayMontage` (`self.Mesh`) "/Game/Game/Animations/OLDSTUFF/RangedEnemy/MageAnims/Montages/Mage_LightningStrike_Montage.Mage_LightningStrike_Montage")
    (:`OnCompleted`
      (`self.AttackEnd` AttackTarget :!label _label))
    (:`OnInterrupted`
      (goto _label))
    (:`OnNotifyBegin`
      (switch `name` _notifyname
        (:`Strike`
          (bind _returnvalue (`|SpawnActorFromClass` "/Game/Game/Combat/Attacks/AOE/BP_AOE_LightningStrike.BP_AOE_LightningStrike_C" (`KismetMathLibrary.MakeTransform` (0.0 0.0 0.0)) "Undefined" "MultiplyWithRoot" null 2.0 AttackTarget false false false null))
          (add `/Game/Game/Combat/Attacks/AOE/BP_AOE_Base.OnAOEOverlapActor` _returnvalue (delegate `OnAOEOverlapActor_Event`)))))))

(event `OnAOEOverlapActor_Event`
  (params (Actor :type "Actor Object Reference"))
  ;[1 1 1] Attacks
  (bind _teamnumber (message `/Game/Game/DamageSystem/BPI_Damageable.GetTeamNumber` Actor))
  (if (!= _teamnumber (`self.Team Number`))
    (message `/Game/Game/DamageSystem/BPI_Damageable.TakeDamage` Actor (make `/Game/Game/DamageSystem/S_DamageInfo` 30.0 "NewEnumerator3" "NewEnumerator1") self)))

(event `GroundSmashAttack`
  (params (AttackTarget :type "Actor Object Reference"))
  ;[1 1 1] Attacks
  (`/Game/Game/Combat/Attacks/BPC_Attacks.GroundSmash` (`self.BPC_Attacks`) (make `/Game/Game/Combat/Attacks/S_AttackInfo` AttackTarget "/Game/Game/Animations/OLDSTUFF/RangedEnemy/MageAnims/Montages/Mage_Slam_Montage.Mage_Slam_Montage" (make `/Game/Game/DamageSystem/S_DamageInfo` 25.0 "NewEnumerator3")) 300.0))

(event `BarrageAttack`
  (params (AttackTarget :type "Actor Object Reference"))
  ;[1 1 1] Attacks
  (`/Game/Game/Combat/Attacks/BPC_Attacks.BarrageMageSpell` (`self.BPC_Attacks`) (make `/Game/Game/Combat/Attacks/S_AttackInfo` AttackTarget "/Game/Game/Animations/OLDSTUFF/RangedEnemy/MageAnims/Montages/Montage_Mage_Barrage_Attack.Montage_Mage_Barrage_Attack" (make `/Game/Game/DamageSystem/S_DamageInfo` 15.0 "NewEnumerator3"))))

(event `BasicAttack`
  (params (AttackTarget :type "Actor Object Reference"))
  ;[1 1 1] Attacks
  (`/Game/Game/Combat/Attacks/BPC_Attacks.BasicMageSpell` (`self.BPC_Attacks`) (make `/Game/Game/Combat/Attacks/S_AttackInfo` AttackTarget "/Game/Game/Animations/OLDSTUFF/RangedEnemy/MageAnims/Montages/Montage_Mage_Spell.Montage_Mage_Spell" (make `/Game/Game/DamageSystem/S_DamageInfo` 20.0 "NewEnumerator2"))))

(fn `GetIdealRange`
  (returns (AttackRadius :type "Float (double-precision)") (DefendRadius :type "Float (double-precision)"))
  (return 500.0 700.0))

(fn `SetMovementSpeed`
  (params (Speed :type "/Game/Game/Characters/Enemy/AI/Enums/E_MovementSpeed Enum" :default "NewEnumerator0"))
  (returns (SpeedValue :type "Float (double-precision)"))
  (return (select `/Game/Game/Characters/Enemy/AI/Enums/E_MovementSpeed` Speed :`NewEnumerator1` 150.0 :`NewEnumerator2` 250.0 :`NewEnumerator3` 400.0)))

(fn `UserConstructionScript`
  (`parent.UserConstructionScript`))