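; BP_Enemy_Ranged is a ranged enemy character that carries a bow but attacks by throwing bombs.
; On BeginPlay it spawns a bow and attaches it to the left hand socket.
; Attack plays a throw montage whose notify calls BPCAttacks to throw a timed explosive, then ends the attack on completion or interruption.
; It overrides movement speeds and ideal range; an arrow draw-and-shoot chain remains in the graph but is never run.
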(event `self.ReceiveBeginPlay`
  (`/Game/Game/Characters/Enemy/AI/BPI_EnemyAI.EquipWeapon`)
  (`parent.ReceiveBeginPlay`))

(event `/Game/Game/Characters/Enemy/AI/BPI_EnemyAI.EquipWeapon`
  ;[1 1 1] Equip
  (bind _returnvalue (`|SpawnActorFromClass` "/Game/Game/Combat/Weapons/BP_Weapon_Bow.BP_Weapon_Bow_C" (`KismetMathLibrary.MakeTransform` (0.0 0.0 0.0)) "Undefined" "MultiplyWithRoot" self null))
  (bind _output_get (set `self.WeaponActor` _returnvalue))
  (`self.K2_AttachToComponent` _output_get (`self.Mesh`) "hand_l_bow_socket" "SnapToTarget" "SnapToTarget" "SnapToTarget" true)
  (`self.OnWeaponEquipped`))

(event `CustomEvent`
  (params (AttackTarget :type "Actor Object Reference")))

(event `/Game/Game/Characters/Enemy/AI/BPI_EnemyAI.Attack`
  (params (AttackTarget :type "Actor Object Reference"))
  (`parent.Attack` AttackTarget)
  (bind _notifyname (`|PlayMontage` (`self.Mesh`) "/Game/Game/Animations/NEWSTUFF/Ranged/Montage/Montage_Throw.Montage_Throw")
    (:`OnCompleted`
      (`self.AttackEnd` AttackTarget :!label _label))
    (:`OnInterrupted`
      (goto _label))
    (:`OnNotifyBegin`
      (switch `name` _notifyname
        (:`Throw`
          (`/Game/Game/Combat/Attacks/BPC_Attacks.ThrowBomb` (`self.BPC_Attacks`) (`KismetMathLibrary.MakeTransform` (`self.K2_GetActorLocation`)) (make `/Game/Game/Combat/Attacks/S_AttackInfo` AttackTarget null (make `/Game/Game/DamageSystem/S_DamageInfo` 50.0 "NewEnumerator3")) 150.0 3.0))))))

(fn `GetIdealRange`
  (returns (AttackRadius :type "Float (double-precision)") (DefendRadius :type "Float (double-precision)"))
  (return 600.0 600.0))

(fn `SetMovementSpeed`
  (params (Speed :type "/Game/Game/Characters/Enemy/AI/Enums/E_MovementSpeed Enum" :default "NewEnumerator0"))
  (returns (SpeedValue :type "Float (double-precision)"))
  (set `CharacterMovementComponent.MaxWalkSpeed` (select `/Game/Game/Characters/Enemy/AI/Enums/E_MovementSpeed` Speed :`NewEnumerator1` 200.0 :`NewEnumerator2` 300.0 :`NewEnumerator3` 500.0 :!type "Float (single-precision)") (`self.CharacterMovement`))
  (return 0.0))

(fn `UserConstructionScript`
  (`parent.UserConstructionScript`))