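; BP_Enemy_Ranged is a bow-wielding enemy character that shoots arrows at its AI attack target.
; On BeginPlay it spawns a bow weapon and attaches it to a left-hand socket.
; Attack plays a shoot montage whose notifies drive ACBowMechanics: Draw spawns the arrow and Shoot fires it from the hand toward the AI controller's target.
; It also supplies movement speeds and ideal attack and defend ranges.
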(event `self.ReceiveBeginPlay`
  (`/Game/Game/Characters/Enemy/AI/BPI_EnemyAI.EquipWeapon`)
  (`parent.ReceiveBeginPlay`))

(event `/Game/Game/Characters/Enemy/AI/BPI_EnemyAI.EquipWeapon`
  ;[1 1 1] Equip
  (bind _returnvalue (`|SpawnActorFromClass` "/Game/Game/Weapons/BP_Weapon_Bow.BP_Weapon_Bow_C" (`KismetMathLibrary.MakeTransform` (0.0 0.0 0.0)) "Undefined" "MultiplyWithRoot" null null))
  (bind _output_get (set `self.WeaponActor` _returnvalue))
  (`self.K2_AttachToComponent` _output_get (`self.Mesh`) "hand_l_bow_socket" "SnapToTarget" "SnapToTarget" "SnapToTarget" true)
  (`self.OnWeaponEquipped`))

(event `/Game/Game/Characters/Enemy/AI/BPI_EnemyAI.Attack`
  (bind _notifyname (`|PlayMontage` (`self.Mesh`) "/Game/Game/Animations/RangedEnemy/Anims/SimpleShoot_Montage.SimpleShoot_Montage")
    (:`OnCompleted`
      (`self.OnAttackEnd` :!label _label))
    (:`OnInterrupted`
      (goto _label))
    (:`OnNotifyBegin`
      (switch `name` _notifyname
        (:`Shoot`
          (bind _asaic_enemy_base (cast `/Game/Game/Characters/Enemy/AI/AIC_Enemy_Base` (`AIBlueprintHelperLibrary.GetAIController` self)))
          (bind _attack_target (`/Game/Game/Characters/Enemy/AI/AIC_Enemy_Base.Attack Target` _asaic_enemy_base)
            (:`then`
              (`/Game/Game/Weapons/AC_BowMechanics.FireArrowBegin` (`self.AC_BowMechanics`) (* (`self.ArrowSpeed`) (`KismetMathLibrary.Normal` (- (`self.K2_GetActorLocation` _attack_target) (`SceneComponent.GetSocketLocation` (`self.Mesh`) "hand_r_arrow_socket"))))))
            (:`else`)))
        (:`Draw`
          (`/Game/Game/Weapons/AC_BowMechanics.SpawnArrow` (`self.AC_BowMechanics`)))))))

(fn `GetIdealRange`
  (returns (AttackRadius :type "Float (double-precision)") (DefendRadius :type "Float (double-precision)"))
  (return 600.0 600.0))

(fn `SetMovementSpeed`
  (params (Speed :type "/Game/Game/Characters/Enemy/AI/Enums/E_MovementSpeed Enum" :default "NewEnumerator0"))
  (returns (SpeedValue :type "Float (double-precision)"))
  (set `CharacterMovementComponent.MaxWalkSpeed` (select `/Game/Game/Characters/Enemy/AI/Enums/E_MovementSpeed` Speed :`NewEnumerator1` 200.0 :`NewEnumerator2` 300.0 :`NewEnumerator3` 500.0 :!type "Float (single-precision)") (`self.CharacterMovement`))
  (return 0.0))

(fn `UserConstructionScript`
  (`parent.UserConstructionScript`))