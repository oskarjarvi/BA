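; Melee enemy character that draws and sheathes a sword and offers short-range, long-range, ground smash and spinning attacks.
; Draw and sheath montage notifies spawn the sword on a hand socket or destroy it, with callbacks signalling when equipping finishes.
; Each attack event passes its montage and damage info to the BPCAttacks component.
; Helpers supply ideal attack and defend ranges and predict an actor's future location from horizontal velocity.
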(event `self.ReceiveBeginPlay`
  (`parent.ReceiveBeginPlay`))

(event `/Game/Game/Characters/Enemy/AI/BPI_EnemyAI.EquipWeapon`
  ;[1 1 1] Equipping Weapon
  (bind _notifyname (`|PlayMontage` (`self.Mesh`) "/Game/Game/Animations/NEWSTUFF/Enemy/Montages/AM_Draw.AM_Draw")
    (:`OnCompleted`
      (`self.OnWeaponEquipped` :!label _label))
    (:`OnInterrupted`
      (goto _label))
    (:`OnNotifyBegin`
      (switch `name` _notifyname
        (:`WieldSword`
          (bind _returnvalue (`|SpawnActorFromClass` "/Game/Game/Combat/Weapons/BP_Weapon_Sword.BP_Weapon_Sword_C" (`self.GetTransform`) "Undefined" "MultiplyWithRoot" self null))
          (bind _output_get (set `self.WeaponActor` _returnvalue))
          (`self.K2_AttachToComponent` _output_get (`self.Mesh`) "hand_r_sword_socket" "SnapToTarget" "SnapToTarget" "SnapToTarget" true)
          (set `self.IsWieldingWeapon` true))))))

(event `/Game/Game/Characters/Enemy/AI/BPI_EnemyAI.UnEquipWeapon`
  ;[1 1 1] Unequipping sword
  (bind _notifyname (`|PlayMontage` (`self.Mesh`) "/Game/Game/Animations/NEWSTUFF/Enemy/Montages/AM_Sheath.AM_Sheath")
    (:`OnCompleted`
      (`self.OnWeaponUnequipped`))
    (:`OnNotifyBegin`
      (switch `name` _notifyname
        (:`UnequipSword`
          (`self.K2_DestroyActor` (`self.WeaponActor`))
          (set `self.IsWieldingWeapon` false))))))

(event `ShortRangeAttack`
  (params (AttackTarget :type "Actor Object Reference"))
  ;[1 1 1] Attacks
  (`/Game/Game/Combat/Attacks/BPC_Attacks.PrimaryMeleeAttack` (`self.BPC_Attacks`) (make `/Game/Game/Combat/Attacks/S_AttackInfo` AttackTarget "/Game/Game/Animations/NEWSTUFF/Enemy/Montages/AM_Slash.AM_Slash" (make `/Game/Game/DamageSystem/S_DamageInfo` 10.0 "NewEnumerator1" "NewEnumerator0" false true true)) 20.0 200.0))

(event `LongRangeAttack`
  (params (AttackTarget :type "Actor Object Reference"))
  ;[1 1 1] Attacks
  (`/Game/Game/Combat/Attacks/BPC_Attacks.LongRangeMeleeAttack` (`self.BPC_Attacks`) (make `/Game/Game/Combat/Attacks/S_AttackInfo` AttackTarget "/Game/Game/Animations/NEWSTUFF/Enemy/Montages/AM_JumpAttack.AM_JumpAttack" (make `/Game/Game/DamageSystem/S_DamageInfo` 10.0 "NewEnumerator1" "NewEnumerator0" false true true))))

(event `GroundSmashAttack`
  (params (AttackTarget :type "Actor Object Reference"))
  ;[1 1 1] Attacks
  (`/Game/Game/Combat/Attacks/BPC_Attacks.GroundSmash` (`self.BPC_Attacks`) (make `/Game/Game/Combat/Attacks/S_AttackInfo` AttackTarget "/Game/Game/Animations/NEWSTUFF/Enemy/Montages/AM_Smash.AM_Smash" (make `/Game/Game/DamageSystem/S_DamageInfo` 25.0 "NewEnumerator3")) 200.0))

(event `SpinningAttack`
  (params (AttackTarget :type "Actor Object Reference"))
  ;[1 1 1] Attacks
  (`/Game/Game/Combat/Attacks/BPC_Attacks.SpinningMeleeAttack` (`self.BPC_Attacks`) (make `/Game/Game/Combat/Attacks/S_AttackInfo` AttackTarget "/Game/Game/Animations/NEWSTUFF/Enemy/Animations/Montage_Sword_SpinAttack.Montage_Sword_SpinAttack" (make `/Game/Game/DamageSystem/S_DamageInfo` 10.0 "NewEnumerator1" "NewEnumerator0" false true))))

(fn `CalculateFutureActorLocation`
  (params (Actor :type "Actor Object Reference") (Time :type "Float (double-precision)"))
  (returns (Location :type "Vector Structure"))
  (return (+ (`self.K2_GetActorLocation` Actor) (* (* (`self.GetVelocity` Actor) (1.0 1.0 0.0)) Time))))

(fn `GetIdealRange`
  (returns (AttackRadius :type "Float (double-precision)") (DefendRadius :type "Float (double-precision)"))
  (return 200.0 400.0))

(fn `UserConstructionScript`
  (`parent.UserConstructionScript`))